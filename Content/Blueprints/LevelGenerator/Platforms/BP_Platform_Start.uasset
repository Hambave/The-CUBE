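; BP_Platform_Start is a level-generator platform, named as the start piece, with color-cycling glow and two kill volumes.
; BeginPlay caches the first BP_Player and creates a dynamic material on Cube5.
; A Delay on Tick throttles random changes to the material's Color parameter, scaled above normal range for bright HDR values.
; Any overlap with Box or Box1 calls Dead on the cached player, without checking the overlapping actor.
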(event OnComponentBeginOverlap(Box1)
  (params (OverlappedComponent :type Primitive%20Component%20Object%20Reference) (OtherActor :type Actor%20Object%20Reference) (OtherComp :type Primitive%20Component%20Object%20Reference) (OtherBodyIndex :type Integer) (bFromSweep :type Boolean) (SweepResult :type Hit%20Result%20Structure%20%28by%20ref%29))
  (Default|Dead (Variables|Default|GetPlayer%20Reference)))

(event OnComponentBeginOverlap(Box)
  (params (OverlappedComponent :type Primitive%20Component%20Object%20Reference) (OtherActor :type Actor%20Object%20Reference) (OtherComp :type Primitive%20Component%20Object%20Reference) (OtherBodyIndex :type Integer) (bFromSweep :type Boolean) (SweepResult :type Hit%20Result%20Structure%20%28by%20ref%29))
  (Default|Dead (Variables|Default|GetPlayer%20Reference)))

(event EventBeginPlay
  (bind _outactors (Actor|GetAllActorsOfClass "/Game/Blueprints/Player/BP_Player.BP_Player_C"))
  (Variables|Default|SetPlayer%20Reference (Utilities|Array|Get(acopy) _outactors))
  (bind _returnvalue (Rendering|Material|CreateDynamicMaterialInstance (Variables|Default|GetCube5) 0 0 "None" :!class /Script/Engine.PrimitiveComponent))
  (bind _output_get (Variables|Default|SetDynamic%20Material _returnvalue))
  (Rendering|Material|SetVectorParameterValue _output_get "Color" (Math|Color|MakeColor (* (Math|Random|RandomFloatinRange 0.0 1.0) 2e+01) (* (Math|Random|RandomFloatinRange 0.0 1.0) 2e+01) (* (Math|Random|RandomFloatinRange 0.0 1.0) 2e+01) 0.0) :!class /Script/Engine.MaterialInstanceDynamic))

(event EventTick
  (params (DeltaSeconds :type Float%20%28single-precision%29))
  (Utilities|FlowControl|Delay 0.3)
  (Rendering|Material|SetVectorParameterValue (stale EventBeginPlay _output_get) "Color" (Math|Color|MakeColor (* (Math|Random|RandomFloatinRange 0.0 1.0) 2e+01) (* (Math|Random|RandomFloatinRange 0.0 1.0) 2e+01) (* (Math|Random|RandomFloatinRange 0.0 1.0) 2e+01) 0.0) :!class /Script/Engine.MaterialInstanceDynamic))

(fn ConstructionScript)