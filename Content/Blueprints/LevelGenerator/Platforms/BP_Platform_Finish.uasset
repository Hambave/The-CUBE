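; BP_Platform_Finish is the finish platform of a generated level, completing the run when its box trigger is overlapped.
; On BeginPlay it caches the first BP_Player and BP_Level_Generator found in the world.
; Any overlap, with no actor check, calls Finish on the player, then increments its easy, medium or hard completed-level counter according to the generator's difficulty flags.
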(event OnComponentBeginOverlap(Box)
  (params (OverlappedComponent :type Primitive%20Component%20Object%20Reference) (OtherActor :type Actor%20Object%20Reference) (OtherComp :type Primitive%20Component%20Object%20Reference) (OtherBodyIndex :type Integer) (bFromSweep :type Boolean) (SweepResult :type Hit%20Result%20Structure%20%28by%20ref%29))
  (bind _level_generator (Variables|Default|GetLevel%20Generator))
  (Default|Finish (Variables|Default|GetPlayer%20Reference))
  (Utilities|FlowControl|Sequence
    (:then_0
      (if (Variables|/Game/Blueprints/LevelGenerator/BP_Level_Generator.BP_Level_Generator_C|GetbEasy _level_generator)
        (Math|Integer|IncrementInt (Variables|/Game/Blueprints/Player/BP_Player.BP_Player_C|GetEasy%20Levels%20Completed (Variables|Default|GetPlayer%20Reference)))))
    (:then_1
      (if (Variables|/Game/Blueprints/LevelGenerator/BP_Level_Generator.BP_Level_Generator_C|GetbMedium _level_generator)
        (Math|Integer|IncrementInt (Variables|/Game/Blueprints/Player/BP_Player.BP_Player_C|GetMedium%20Levels%20Completed (Variables|Default|GetPlayer%20Reference)))))
    (:then_2
      (if (Variables|/Game/Blueprints/LevelGenerator/BP_Level_Generator.BP_Level_Generator_C|GetbHard _level_generator)
        (Math|Integer|IncrementInt (Variables|/Game/Blueprints/Player/BP_Player.BP_Player_C|GetHard%20Levels%20Completed (Variables|Default|GetPlayer%20Reference)))))))

(event EventBeginPlay
  (bind _outactors (Actor|GetAllActorsOfClass "/Game/Blueprints/Player/BP_Player.BP_Player_C"))
  (Variables|Default|SetPlayer%20Reference (Utilities|Array|Get(acopy) _outactors))
  (bind _outactors_2 (Actor|GetAllActorsOfClass "/Game/Blueprints/LevelGenerator/BP_Level_Generator.BP_Level_Generator_C"))
  (Variables|Default|SetLevel%20Generator (Utilities|Array|Get(acopy) _outactors_2)))

(fn ConstructionScript)