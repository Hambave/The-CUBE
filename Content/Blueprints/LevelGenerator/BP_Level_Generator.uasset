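; Level generator actor that builds a randomly branching path of platforms for preset-difficulty or endless runs.
; Difficulty flags set level length and player speed, while endless mode takes its speed from the player controller.
; Generation removes the main menu, then chains platforms at random unoccupied attachment points on the last one, ending finite levels with a finish platform.
; In endless mode, Tick extends the chain whenever the player nears its end.
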(event Custom|Setup%20Difficulty
  (bind _player_reference (Variables|Default|GetPlayer%20Reference))
  (Utilities|FlowControl|Sequence
    (:then_0
      (if (Variables|Default|GetbEasy)
        (Variables|Default|SetLevel%20Lenght 100)
        (Variables|/Game/Blueprints/Player/BP_Player.BP_Player_C|SetSpeed _player_reference 0.28)))
    (:then_1
      (if (Variables|Default|GetbMedium)
        (Variables|Default|SetLevel%20Lenght 300)
        (Variables|/Game/Blueprints/Player/BP_Player.BP_Player_C|SetSpeed _player_reference 0.2)))
    (:then_2
      (if (Variables|Default|GetbHard)
        (Variables|Default|SetLevel%20Lenght 500)
        (Variables|/Game/Blueprints/Player/BP_Player.BP_Player_C|SetSpeed _player_reference 0.15)))
    (:then_3
      (if (Variables|Default|GetbEndless%20Level?)
        (Variables|/Game/Blueprints/Player/BP_Player.BP_Player_C|SetSpeed _player_reference (Variables|/Game/Blueprints/Player/BP_Player_Controller.BP_Player_Controller_C|GetSpeed (Variables|Default|GetPlayer%20Controller)))))))

(event Custom|Generate%20Level
  (Widget|RemovefromParent (Variables|/Game/Blueprints/Player/BP_Player_Controller.BP_Player_Controller_C|GetMain%20Menu%20HUD (Variables|Default|GetPlayer%20Controller)))
  (bind _returnvalue (Game|SpawnActorfromClass "/Game/Blueprints/LevelGenerator/Platforms/BP_Platform_Main.BP_Platform_Main_C" (Math|Transform|MakeTransform "767.475525,-25.213366,1050.000000" "0,180.000000, 0" "1.000000,1.000000,1.000000") "Undefined" 0 0))
  (Variables|Default|SetPlatform%20Reference _returnvalue)
  (for _index (range 1 (Variables|Default|GetLevel%20Lenght))
    (bind _output_get (Variables|Default|SetRandom%20Point (.OutItem (Utilities|Array|Random (Utilities|Array|MakeArray (Variables|/Game/Blueprints/LevelGenerator/Platforms/BP_Platform_Main.BP_Platform_Main_C|GetBox1 (Variables|Default|GetPlatform%20Reference)) (Variables|/Game/Blueprints/LevelGenerator/Platforms/BP_Platform_Main.BP_Platform_Main_C|GetBox2 (Variables|Default|GetPlatform%20Reference)) (Variables|/Game/Blueprints/LevelGenerator/Platforms/BP_Platform_Main.BP_Platform_Main_C|GetBox3 (Variables|Default|GetPlatform%20Reference)))))))
    (if (not (Utilities|Array|IsNotEmpty (Collision|GetOverlappingActors _output_get 0 :!class /Script/Engine.PrimitiveComponent)))
      (bind _returnvalue_2 (Game|SpawnActorfromClass "/Game/Blueprints/LevelGenerator/Platforms/BP_Platform_Main.BP_Platform_Main_C" (Math|Transform|MakeTransform (Transformation|GetWorldLocation (Variables|Default|GetRandom%20Point)) (.rotation (Transformation|GetActorTransform (Variables|Default|GetPlatform%20Reference))) (.scale (Transformation|GetActorTransform (Variables|Default|GetPlatform%20Reference)))) "AlwaysSpawn" 0 0))
      (Variables|Default|SetPlatform%20Reference _returnvalue_2)))
  (if (not (Variables|Default|GetbEndless%20Level?))
    (Game|SpawnActorfromClass "/Game/Blueprints/LevelGenerator/Platforms/BP_Platform_Finish.BP_Platform_Finish_C" (Math|Transform|MakeTransform (Transformation|GetWorldLocation (Variables|/Game/Blueprints/LevelGenerator/Platforms/BP_Platform_Main.BP_Platform_Main_C|GetBox2 (Variables|Default|GetPlatform%20Reference))) "0, 0, 0" "1.000000,1.000000,1.000000") "AlwaysSpawn" 0 0)))

(event EventBeginPlay
  (bind _outactors (Actor|GetAllActorsOfClass "/Game/Blueprints/Player/BP_Player.BP_Player_C"))
  (Variables|Default|SetPlayer%20Reference (Utilities|Array|Get(acopy) _outactors))
  (bind _asbp_player_controller (Utilities|Casting|CastToBP_Player_Controller (Game|GetPlayerController 0)))
  (Variables|Default|SetPlayer%20Controller _asbp_player_controller))

(event EventTick
  (params (DeltaSeconds :type Float%20%28single-precision%29))
  (if (Variables|Default|GetbEndless%20Level?)
    (if (not (> (Math|Vector|VectorLength (- (Transformation|GetWorldLocation (Variables|/Script/Engine.Actor|GetRootComponent (Variables|Default|GetPlayer%20Reference))) (Transformation|GetWorldLocation (Variables|/Game/Blueprints/LevelGenerator/Platforms/BP_Platform_Main.BP_Platform_Main_C|GetCube (Variables|Default|GetPlatform%20Reference))))) 4e+03))
      (for _index (range 1 2)
        (bind _output_get (Variables|Default|SetRandom%20Point (.OutItem (Utilities|Array|Random (Utilities|Array|MakeArray (Variables|/Game/Blueprints/LevelGenerator/Platforms/BP_Platform_Main.BP_Platform_Main_C|GetBox1 (Variables|Default|GetPlatform%20Reference)) (Variables|/Game/Blueprints/LevelGenerator/Platforms/BP_Platform_Main.BP_Platform_Main_C|GetBox2 (Variables|Default|GetPlatform%20Reference)) (Variables|/Game/Blueprints/LevelGenerator/Platforms/BP_Platform_Main.BP_Platform_Main_C|GetBox3 (Variables|Default|GetPlatform%20Reference)))))))
        (if (not (Utilities|Array|IsNotEmpty (Collision|GetOverlappingActors _output_get 0 :!class /Script/Engine.PrimitiveComponent)))
          (bind _returnvalue (Game|SpawnActorfromClass "/Game/Blueprints/LevelGenerator/Platforms/BP_Platform_Main.BP_Platform_Main_C" (Math|Transform|MakeTransform (Transformation|GetWorldLocation (Variables|Default|GetRandom%20Point)) (.rotation (Transformation|GetActorTransform (Variables|Default|GetPlatform%20Reference))) (.scale (Transformation|GetActorTransform (Variables|Default|GetPlatform%20Reference)))) "AlwaysSpawn" 0 0))
          (Variables|Default|SetPlatform%20Reference _returnvalue))))))

(fn ConstructionScript)