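; Test platform actor for a generated level with randomized cube color and side triggers that kill the player.
; BeginPlay caches the level generator and player, while a delayed Tick rerolls the dynamic material color about every second.
; The first Box overlap recolors the cube and adds score in endless levels; End4–6 overlaps call Dead.
; Construction toggles damage text; platform spawning, edge collision and cleanup logic are disconnected.
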(event OnComponentBeginOverlap(Box)
  (params (OverlappedComponent :type Primitive%20Component%20Object%20Reference) (OtherActor :type Actor%20Object%20Reference) (OtherComp :type Primitive%20Component%20Object%20Reference) (OtherBodyIndex :type Integer) (bFromSweep :type Boolean) (SweepResult :type Hit%20Result%20Structure%20%28by%20ref%29))
  (Utilities|FlowControl|DoOnce false
    (:Completed
      (Utilities|FlowControl|Sequence
        (:then_0
          (bind _returnvalue (Rendering|Material|CreateDynamicMaterialInstance (Variables|Default|GetCube1) 0 0 "None" :!class /Script/Engine.PrimitiveComponent))
          (bind _output_get (Variables|Default|SetDynamic%20Material _returnvalue))
          (Rendering|Material|SetVectorParameterValue _output_get "Color" (Math|Color|MakeColor (Math|Random|RandomFloatinRange 0.0 15.0) (Math|Random|RandomFloatinRange 0.0 15.0) (Math|Random|RandomFloatinRange 0.0 15.0) 0.0) :!class /Script/Engine.MaterialInstanceDynamic))
        (:then_1
          (if (Variables|/Game/Blueprints/BP_Level_Generator.BP_Level_Generator_C|GetbEndless%20Level? (Variables|Default|GetLevel%20Generator%20Reference))
            (Math|Integer|IncrementInt (Variables|/Game/Blueprints/Player/BP_Player.BP_Player_C|GetScore (Variables|Default|GetPlayer%20Character)))))))))

(event OnComponentBeginOverlap(End4)
  (params (OverlappedComponent :type Primitive%20Component%20Object%20Reference) (OtherActor :type Actor%20Object%20Reference) (OtherComp :type Primitive%20Component%20Object%20Reference) (OtherBodyIndex :type Integer) (bFromSweep :type Boolean) (SweepResult :type Hit%20Result%20Structure%20%28by%20ref%29))
  (bind _player_character (Variables|Default|GetPlayer%20Character))
  (if (not (Variables|/Game/Blueprints/Player/BP_Player.BP_Player_C|GetbDead _player_character))
    (Default|Dead _player_character)))

(event OnComponentBeginOverlap(End5)
  (params (OverlappedComponent :type Primitive%20Component%20Object%20Reference) (OtherActor :type Actor%20Object%20Reference) (OtherComp :type Primitive%20Component%20Object%20Reference) (OtherBodyIndex :type Integer) (bFromSweep :type Boolean) (SweepResult :type Hit%20Result%20Structure%20%28by%20ref%29))
  (bind _player_character (Variables|Default|GetPlayer%20Character))
  (if (not (Variables|/Game/Blueprints/Player/BP_Player.BP_Player_C|GetbDead _player_character))
    (Default|Dead _player_character)))

(event OnComponentBeginOverlap(End6)
  (params (OverlappedComponent :type Primitive%20Component%20Object%20Reference) (OtherActor :type Actor%20Object%20Reference) (OtherComp :type Primitive%20Component%20Object%20Reference) (OtherBodyIndex :type Integer) (bFromSweep :type Boolean) (SweepResult :type Hit%20Result%20Structure%20%28by%20ref%29))
  (bind _player_character (Variables|Default|GetPlayer%20Character))
  (if (not (Variables|/Game/Blueprints/Player/BP_Player.BP_Player_C|GetbDead _player_character))
    (Default|Dead _player_character)))

(event EventBeginPlay
  (Utilities|FlowControl|Sequence
    (:then_0
      (bind _outactors (Actor|GetAllActorsOfClass "/Game/Blueprints/BP_Level_Generator.BP_Level_Generator_C"))
      (Variables|Default|SetLevel%20Generator%20Reference (Utilities|Array|Get(acopy) _outactors))
      (bind _outactors_2 (Actor|GetAllActorsOfClass "/Game/Blueprints/Player/BP_Player.BP_Player_C"))
      (Variables|Default|SetPlayer%20Character (Utilities|Array|Get(acopy) _outactors_2)))
    (:then_1
      (bind _returnvalue (Rendering|Material|CreateDynamicMaterialInstance (Variables|Default|GetCube1) 0 0 "None" :!class /Script/Engine.PrimitiveComponent))
      (bind _output_get (Variables|Default|SetDynamic%20Material _returnvalue))
      (Rendering|Material|SetVectorParameterValue _output_get "Color" (Math|Color|MakeColor (Math|Random|RandomFloatinRange 0.0 15.0) (Math|Random|RandomFloatinRange 0.0 15.0) (Math|Random|RandomFloatinRange 0.0 15.0) 0.0) :!class /Script/Engine.MaterialInstanceDynamic))))

(event EventTick
  (params (DeltaSeconds :type Float%20%28single-precision%29))
  (Utilities|FlowControl|Delay 1.0)
  (Rendering|Material|SetVectorParameterValue (stale OnComponentBeginOverlap(Box) _output_get) "Color" (Math|Color|MakeColor (Math|Random|RandomFloatinRange 0.0 15.0) (Math|Random|RandomFloatinRange 0.0 15.0) (Math|Random|RandomFloatinRange 0.0 15.0) 0.0) :!class /Script/Engine.MaterialInstanceDynamic))

(fn ConstructionScript
  (bind _textrender (Variables|Default|GetTextRender))
  (Utilities|FlowControl|Sequence
    (:then_0
      (if (Variables|Default|GetbDamage)
        (Development|SetHiddeninGame _textrender false false)
        (else
          (Development|SetHiddeninGame _textrender true false))))))