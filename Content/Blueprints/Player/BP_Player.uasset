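; Player cube that rolls continuously in the last pressed direction (forward, left or right; backward is disabled).
; Tick starts each step as two chained MoveComponentTo arcs, gated by Moving.
; While moving, the dynamic material's color shifts toward red, and endless levels shorten step duration to speed it up.
; Death saves the high score, enables physics and reloads MainLevel, while Finish halts new steps and increments the difficulty's completion counter.
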(event Custom|Dead
  (Utilities|FlowControl|DoOnce false
    (:Completed
      (if (> (Variables|Default|GetScore) (Variables|/Game/Blueprints/Player/BP_Player_Controller.BP_Player_Controller_C|GetHigh%20Score (Variables|Default|GetPlayer%20Controller)))
        (Variables|/Game/Blueprints/Player/BP_Player_Controller.BP_Player_Controller_C|SetHigh%20Score (Variables|Default|GetPlayer%20Controller) (Variables|Default|GetScore)))
      (Variables|Default|SetbDead true)
      (CallFunction|Stop)
      (Physics|SetSimulatePhysics (Variables|Default|GetCube) true)
      (Utilities|FlowControl|Delay 0.5)
      (Game|OpenLevel(byName) "MainLevel"))))

(event Custom|Stop
  (bind _returnvalue (Transformation|GetActorTransform))
  (bind _returnvalue_2 (Transformation|GetActorTransform))
  (bind _returnvalue_3 (Transformation|GetActorTransform))
  (bind _returnvalue_4 (Transformation|GetActorTransform))
  (bind _returnvalue_5 (Transformation|GetActorTransform))
  (bind _returnvalue_6 (Transformation|GetActorTransform))
  (bind (_x _y _z) (Math|Vector|BreakVector (.location _returnvalue_4)))
  (bind (_x_2 _y_2 _z_2) (Math|Vector|BreakVector (.location _returnvalue)))
  (bind (_x_3 _y_3 _z_3) (Math|Vector|BreakVector (.location _returnvalue_3)))
  (bind (_x_4 _y_4 _z_4) (Math|Vector|BreakVector (.location _returnvalue_2)))
  (bind (_x_5 _y_5 _z_5) (Math|Vector|BreakVector (.location _returnvalue_5)))
  (bind (_x_6 _y_6 _z_6) (Math|Vector|BreakVector (.location _returnvalue_6)))
  (Utilities|FlowControl|Sequence
    (:then_0
      (Components|MoveComponentTo (Variables|Default|GetCube) (Math|Vector|MakeVector (+ _x_5 6e+01) _y_5 (+ _z_5 (Variables|Default|GetZ))) "-90.000000,0.000000,0.000000" false false (Variables|Default|GetSpeed) true) ; enters at Stop
    )
    (:then_1
      (Components|MoveComponentTo (Variables|Default|GetCube) (Math|Vector|MakeVector (+ _x_6 6e+01) _y_6 (- _z_6 (Variables|Default|GetZ))) "-0.000000,180.000000,180.000000" false false (Variables|Default|GetSpeed) true) ; enters at Stop
    )
    (:then_2
      (Components|MoveComponentTo (Variables|Default|GetCube) (Math|Vector|MakeVector _x (+ _y -6e+01) (+ _z (Variables|Default|GetZ))) "0.000000,0.000000,-90.000000" false false (Variables|Default|GetSpeed) true) ; enters at Stop
    )
    (:then_3
      (Components|MoveComponentTo (Variables|Default|GetCube) (Math|Vector|MakeVector _x_2 (+ _y_2 -6e+01) (- _z_2 (Variables|Default|GetZ))) "-0.000000,0.000000,-180.000000" false false (Variables|Default|GetSpeed) true) ; enters at Stop
    )
    (:then_4
      (Components|MoveComponentTo (Variables|Default|GetCube) (Math|Vector|MakeVector _x_4 (+ _y_4 6e+01) (- _z_4 (Variables|Default|GetZ))) "-0.000000,0.000000,180.000000" false false (Variables|Default|GetSpeed) true) ; enters at Stop
    )
    (:then_5
      (Components|MoveComponentTo (Variables|Default|GetCube) (Math|Vector|MakeVector _x_3 (+ _y_3 6e+01) (+ _z_3 (Variables|Default|GetZ))) "0.000000,0.000000,90.000000" false false (Variables|Default|GetSpeed) true) ; enters at Stop
    )))

(event Custom|Finish
  (bind _level_generator (Variables|Default|GetLevel%20Generator))
  (Variables|Default|SetbFinished true)
  (Variables|/Script/Engine.PlayerController|SetbShowMouseCursor (Variables|Default|GetPlayer%20Controller) true)
  (Utilities|FlowControl|Sequence
    (:then_0
      (if (Variables|/Game/Blueprints/BP_Level_Generator.BP_Level_Generator_C|GetbEasy _level_generator)
        (Math|Integer|IncrementInt (Variables|Default|GetEasy%20Levels%20Completed))))
    (:then_1
      (if (Variables|/Game/Blueprints/BP_Level_Generator.BP_Level_Generator_C|GetbMedium _level_generator)
        (Math|Integer|IncrementInt (Variables|Default|GetMedium%20Levels%20Completed))))
    (:then_2
      (if (Variables|/Game/Blueprints/BP_Level_Generator.BP_Level_Generator_C|GetbHard _level_generator)
        (Math|Integer|IncrementInt (Variables|Default|GetHard%20Levels%20Completed))))))

(event EventBeginPlay
  (bind _returnvalue (Game|GetPlayerController 0))
  (bind _outactors (Actor|GetAllActorsOfClass "/Game/Blueprints/BP_Level_Generator.BP_Level_Generator_C"))
  (Variables|Default|SetLevel%20Generator (Utilities|Array|Get(acopy) _outactors))
  (Variables|/Script/Engine.PlayerController|SetbShowMouseCursor _returnvalue true)
  (bind _asbp_player_controller (Utilities|Casting|CastToBP_Player_Controller _returnvalue))
  (Variables|Default|SetPlayer%20Controller _asbp_player_controller)
  (bind _returnvalue_2 (Rendering|Material|CreateDynamicMaterialInstance (Variables|Default|GetCube1) 0 0 "None" :!class /Script/Engine.PrimitiveComponent))
  (bind _output_get (Variables|Default|SetDynamicCubeMaterial _returnvalue_2))
  (Rendering|Material|SetScalarParameterValue _output_get "Saturation" 0.5 :!class /Script/Engine.MaterialInstanceDynamic)
  (Rendering|Material|SetVectorParameterValue _output_get "Color" (Math|Color|MakeColor 2e+01 2e+01 2e+01) :!class /Script/Engine.MaterialInstanceDynamic))

(event EventTick
  (params (DeltaSeconds :type Float%20%28single-precision%29))
  (bind _returnvalue (Transformation|GetActorTransform))
  (bind _returnvalue_2 (Transformation|GetActorTransform))
  (bind _returnvalue_3 (Transformation|GetActorTransform))
  (bind _returnvalue_4 (Transformation|GetActorTransform))
  (bind _returnvalue_5 (Transformation|GetActorTransform))
  (bind _returnvalue_6 (Transformation|GetActorTransform))
  (bind (_x _y _z) (Math|Vector|BreakVector (.location _returnvalue_4)))
  (bind (_x_2 _y_2 _z_2) (Math|Vector|BreakVector (.location _returnvalue)))
  (bind (_x_3 _y_3 _z_3) (Math|Vector|BreakVector (.location _returnvalue_3)))
  (bind (_x_4 _y_4 _z_4) (Math|Vector|BreakVector (.location _returnvalue_2)))
  (bind (_x_5 _y_5 _z_5) (Math|Vector|BreakVector (.location _returnvalue_5)))
  (bind (_x_6 _y_6 _z_6) (Math|Vector|BreakVector (.location _returnvalue_6)))
  (if (not (Variables|Default|GetbDead))
    (if (not (Variables|Default|GetbFinished))
      (Rendering|Material|SetScalarParameterValue (Variables|Default|GetDynamicCubeMaterial) "Saturation" 1.0 :!class /Script/Engine.MaterialInstanceDynamic)
      (Utilities|FlowControl|Sequence
        (:then_0
          (if (Variables|Default|GetForward)
            (if (not (Variables|Default|GetbMoving))
              (Variables|Default|SetbMoving true)
              (Components|MoveComponentTo (Variables|Default|GetCube) (Math|Vector|MakeVector (+ _x_5 6e+01) _y_5 (+ _z_5 (Variables|Default|GetZ))) "-90.000000,0.000000,0.000000" false false (Variables|Default|GetSpeed) true)
              (Components|MoveComponentTo (Variables|Default|GetCube) (Math|Vector|MakeVector (+ _x_6 6e+01) _y_6 (- _z_6 (Variables|Default|GetZ))) "-0.000000,180.000000,180.000000" false false (Variables|Default|GetSpeed) true)
              (Transformation|SetRelativeRotation (Variables|Default|GetCube) "0, 0, 0" false false)
              (Variables|Default|SetbMoving false))))
        (:then_1
          (if (Variables|Default|GetLeft)
            (if (not (Variables|Default|GetbMoving))
              (Variables|Default|SetbMoving true)
              (Components|MoveComponentTo (Variables|Default|GetCube) (Math|Vector|MakeVector _x (+ _y -6e+01) (+ _z (Variables|Default|GetZ))) "0.000000,0.000000,-90.000000" false false (Variables|Default|GetSpeed) true)
              (Components|MoveComponentTo (Variables|Default|GetCube) (Math|Vector|MakeVector _x_2 (+ _y_2 -6e+01) (- _z_2 (Variables|Default|GetZ))) "-0.000000,0.000000,-180.000000" false false (Variables|Default|GetSpeed) true)
              (Transformation|SetRelativeRotation (Variables|Default|GetCube) "0, 0, 0" false false)
              (Variables|Default|SetbMoving false))))
        (:then_2
          (if (Variables|Default|GetRight)
            (if (not (Variables|Default|GetbMoving))
              (Variables|Default|SetbMoving true)
              (Components|MoveComponentTo (Variables|Default|GetCube) (Math|Vector|MakeVector _x_3 (+ _y_3 6e+01) (+ _z_3 (Variables|Default|GetZ))) "0.000000,0.000000,90.000000" false false (Variables|Default|GetSpeed) true)
              (Components|MoveComponentTo (Variables|Default|GetCube) (Math|Vector|MakeVector _x_4 (+ _y_4 6e+01) (- _z_4 (Variables|Default|GetZ))) "-0.000000,0.000000,180.000000" false false (Variables|Default|GetSpeed) true)
              (Transformation|SetRelativeRotation (Variables|Default|GetCube) "0, 0, 0" false false)
              (Variables|Default|SetbMoving false))))
        (:then_3
          (|UpTheSpeedOverCertainTime))
        (:then_4
          (|ChangeCubeSaturationOverTime))))))

(event Input|ActionEvents|InputActionRight
  (params (Key :type Key%20Structure :default "None"))
  (:Pressed
    (if (not (Variables|Default|GetbDead))
      (Variables|Default|SetBackward false)
      (Variables|Default|SetForward false)
      (Variables|Default|SetLeft false)
      (Variables|Default|SetRight true))))

(event Input|ActionEvents|InputActionLeft
  (params (Key :type Key%20Structure :default "None"))
  (:Pressed
    (if (not (Variables|Default|GetbDead))
      (Variables|Default|SetBackward false)
      (Variables|Default|SetRight false)
      (Variables|Default|SetForward false)
      (Variables|Default|SetLeft true))))

(event Input|ActionEvents|InputActionForward
  (params (Key :type Key%20Structure :default "None"))
  (:Pressed
    (if (not (Variables|Default|GetbDead))
      (Variables|Default|SetLeft false)
      (Variables|Default|SetBackward false)
      (Variables|Default|SetRight false)
      (Variables|Default|SetForward true))))

(event Input|KeyboardEvents|S
  (params (Key :type Key%20Structure :default "None")))

(fn ConstructionScript)