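; Player controller that creates the main menu and player HUD widgets and manages persistence of the high score and sound setting.
; On BeginPlay it loads the SaveGameCUBE slot into HighScore and the menu's Sound flag, or creates and saves a new one.
; It then sets the pawn's landing sound volume from that flag, only at startup.
; Tick copies both values back and writes the save to disk every frame.
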(event EventBeginPlay
  (bind _asbp_player (Utilities|Casting|CastToBP_Player (Game|Player|GetPlayerPawn 0)))
  (Variables|Default|SetPlayer%20Reference _asbp_player)
  (bind _returnvalue (UserInterface|CreateWidget "/Game/Blueprints/HUDs/BP_MainMenu_HUD.BP_MainMenu_HUD_C"))
  (bind _output_get (Variables|Default|SetMain%20Menu%20HUD _returnvalue))
  (UserInterface|Viewport|AddtoViewport _output_get 0)
  (bind _returnvalue_2 (UserInterface|CreateWidget "/Game/Blueprints/HUDs/BP_Player_HUD.BP_Player_HUD_C"))
  (bind _output_get_2 (Variables|Default|SetPlayer%20HUD _returnvalue_2))
  (UserInterface|Viewport|AddtoViewport _output_get_2 0)
  (Utilities|FlowControl|Sequence
    (:then_0
      (bind _returnvalue_3 (SaveGame|DoesSaveGameExist "1"))
      (if _returnvalue_3
        (bind _returnvalue_4 (SaveGame|LoadGamefromSlot "1"))
        (bind _assave_game_cube (Utilities|Casting|CastToSaveGameCUBE _returnvalue_4))
        (Variables|Default|SetSave%20Game _assave_game_cube)
        (CallFunction|LoadandSetVar)
        (else
          (bind _returnvalue_5 (SaveGame|CreateSaveGameObject "/Game/Blueprints/SaveGameCUBE.SaveGameCUBE_C"))
          (bind _output_get_3 (Variables|Default|SetSave%20Game _returnvalue_5))
          (SaveGame|SaveGametoSlot _output_get_3 "1"))))
    (:then_1
      (if (Variables|/Game/Blueprints/HUDs/BP_MainMenu_HUD.BP_MainMenu_HUD_C|GetSound (Variables|Default|GetMain%20Menu%20HUD))
        (Audio|Components|Audio|SetVolumeMultiplier (Variables|/Game/Blueprints/Player/BP_Player.BP_Player_C|GetLanding_Sound_Cue (Variables|Default|GetPlayer%20Reference)) 1.0 :!class /Script/Engine.AudioComponent)
        (else
          (Audio|Components|Audio|SetVolumeMultiplier (Variables|/Game/Blueprints/Player/BP_Player.BP_Player_C|GetLanding_Sound_Cue (Variables|Default|GetPlayer%20Reference)) 0.0 :!class /Script/Engine.AudioComponent))))))

(event EventTick
  (params (DeltaSeconds :type Float%20%28single-precision%29))
  (bind _save_game (Variables|Default|GetSave%20Game))
  (Variables|/Game/Blueprints/SaveGameCUBE.SaveGameCUBE_C|SetSound _save_game (Variables|/Game/Blueprints/HUDs/BP_MainMenu_HUD.BP_MainMenu_HUD_C|GetSound (Variables|Default|GetMain%20Menu%20HUD)))
  (Variables|/Game/Blueprints/SaveGameCUBE.SaveGameCUBE_C|SetHigh%20Score _save_game (Variables|Default|GetHigh%20Score))
  (SaveGame|SaveGametoSlot (stale EventBeginPlay _output_get_3) "1"))

(fn ConstructionScript)

(fn LoadandSetVar
  (bind _save_game (Variables|Default|GetSave%20Game))
  (Variables|Default|SetHigh%20Score (Variables|/Game/Blueprints/SaveGameCUBE.SaveGameCUBE_C|GetHigh%20Score _save_game))
  (Variables|/Game/Blueprints/HUDs/BP_MainMenu_HUD.BP_MainMenu_HUD_C|SetSound (Variables|Default|GetMain%20Menu%20HUD) (Variables|/Game/Blueprints/SaveGameCUBE.SaveGameCUBE_C|GetSound _save_game)))